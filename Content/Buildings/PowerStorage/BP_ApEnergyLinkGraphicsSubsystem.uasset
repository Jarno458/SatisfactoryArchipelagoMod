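; Subsystem for the Ap EnergyLink graphics that adds an overlay to the power storage UI.
; On BeginPlay it hooks the Construct function of BPW_PowerStorage through a Blueprint function binding, leaving that widget's asset untouched.
; Each time the hook fires, it creates a Widget_PowerStorage_ApOverlay and adds it to the CanvasPanel parenting the power circuit graph, logging an error if that parent is another type.
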(event Custom|On%20BPW%20Power%20Storage%20Construct
  (params (Object :type Object%20Object%20Reference))
  (bind _asbpw_power_storage (Utilities|Casting|CastToBPW_PowerStorage Object))
  (Class|BlueprintLoggingLibrary|LogVerbose (Utilities|String|Append "Modifying power storage widget " (Utilities|GetDisplayName _asbpw_power_storage)))
  (Utilities|FlowControl|Sequence
    (:then_0
      (bind _ascanvas_panel (Utilities|Casting|CastToCanvasPanel (Widget|GetParent (Variables|/Game/FactoryGame/Buildable/Factory/PowerStorage/UI/BPW_PowerStorage.BPW_PowerStorage_C|GetmPowerCircuitGraph _asbpw_power_storage)))
        (:then
          (bind _returnvalue (UserInterface|CreateWidget "/Archipelago/Buildings/PowerStorage/Widget_PowerStorage_ApOverlay.Widget_PowerStorage_ApOverlay_C"))
          (Class|CanvasPanel|AddChildtoCanvas _ascanvas_panel _returnvalue))
        (:CastFailed
          (Class|BlueprintLoggingLibrary|LogError "mPowerCircuitGraph Parent not CanvasPanel?"))))))

(event EventBeginPlay
  (Class|BlueprintLoggingLibrary|LogVerbose "ApEnergyLinkGraphicsSubsystem begin")
  (Class|RuntimeBlueprintFunctionLibrary|BindonBPFunction "/Game/FactoryGame/Buildable/Factory/PowerStorage/UI/BPW_PowerStorage.BPW_PowerStorage_C" (delegate Custom|On%20BPW%20Power%20Storage%20Construct) "Construct" false))

(fn ConstructionScript)