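; Decor subsystem that swaps monitor screen materials on the Hub terminal, MAM, Space Elevator and Trading Post for Archipelago-branded versions.
; On BeginPlay, and whenever a relevant buildable is constructed, it starts a one-second looping timer that stops after a maximum tick count.
; Each tick scans those actors and replaces only stock screen materials, using a mesh-to-slot map for Trading Post stages.
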(event Custom|On%20Buildable%20Constructed
  (params (buildable :type FG%20Buildable%20Object%20Reference))
  (if (Utilities|Set|Contains (Variables|Default|GetRelevant%20Buildables) (Utilities|GetClass buildable))
    (Class|BlueprintLoggingLibrary|LogVerbose (Utilities|String|Append "Relevant buildable so starting timer: " (Utilities|GetDisplayName buildable)))
    (Variables|Default|SetTimer%20Ticks 0)
    (bind _returnvalue (Utilities|Time|SetTimerbyEvent (delegate Custom|Material%20Replacer%20Timer%20Tick) 1.0 true))
    (Variables|Default|SetTimer%20Handle _returnvalue)))

(event Custom|Material%20Replacer%20Timer%20Tick
  (bind _returnvalue (Class|KismetSystemLibrary|MakeLiteralInteger 3))
  (bind _returnvalue_2 (Class|KismetSystemLibrary|MakeLiteralInteger 3))
  (bind _returnvalue_3 (Class|KismetSystemLibrary|MakeLiteralInteger 3))
  (Utilities|FlowControl|Sequence
    (:then_0
      (bind _outactors (Actor|GetAllActorsOfClass "/Game/FactoryGame/Buildable/Factory/HubTerminal/Build_HubTerminal.Build_HubTerminal_C"))
      (for _array_element _outactors
        (if (== (Rendering|Material|GetMaterial (Variables|/Game/FactoryGame/Buildable/Factory/HubTerminal/Build_HubTerminal.Build_HubTerminal_C|GetMainMesh _array_element) _returnvalue_2) "/Game/FactoryGame/Buildable/Factory/TradingPost/Material/Monitor_Hub.Monitor_Hub")
          (Rendering|Material|SetMaterial (Variables|/Game/FactoryGame/Buildable/Factory/HubTerminal/Build_HubTerminal.Build_HubTerminal_C|GetMainMesh _array_element) _returnvalue_2 "/Archipelago/Assets/DerivedArt/Decor/MI_Monitor_ArchipelagoHub.MI_Monitor_ArchipelagoHub"))))
    (:then_1
      (bind _outactors_2 (Actor|GetAllActorsOfClass "/Game/FactoryGame/Buildable/Factory/Mam/Build_Mam.Build_Mam_C"))
      (for _array_element_2 _outactors_2
        (if (== (Rendering|Material|GetMaterial (Variables|/Game/FactoryGame/Buildable/Factory/Mam/Build_Mam.Build_Mam_C|GetMainMesh_static _array_element_2) _returnvalue_3) "/Game/FactoryGame/Buildable/Factory/TradingPost/Material/Monitor_MAM.Monitor_MAM")
          (Rendering|Material|SetMaterial (Variables|/Game/FactoryGame/Buildable/Factory/Mam/Build_Mam.Build_Mam_C|GetMainMesh_static _array_element_2) _returnvalue_3 "/Archipelago/Assets/DerivedArt/Decor/MI_Monitor_ArchipelagoMAM.MI_Monitor_ArchipelagoMAM"))))
    (:then_2
      (bind _outactors_3 (Actor|GetAllActorsOfClass "/Game/FactoryGame/Buildable/Factory/SpaceElevator/Build_SpaceElevator.Build_SpaceElevator_C"))
      (for _array_element_3 _outactors_3
        (if (== (Rendering|Material|GetMaterial (Variables|/Game/FactoryGame/Buildable/Factory/SpaceElevator/Build_SpaceElevator.Build_SpaceElevator_C|GetMainMesh _array_element_3) _returnvalue) "/Game/FactoryGame/Buildable/Factory/TradingPost/Material/Monitor_SpaceElevator.Monitor_SpaceElevator")
          (Rendering|Material|SetMaterial (Variables|/Game/FactoryGame/Buildable/Factory/SpaceElevator/Build_SpaceElevator.Build_SpaceElevator_C|GetMainMesh _array_element_3) _returnvalue "/Archipelago/Assets/DerivedArt/Decor/MI_Monitor_ArchipelagoSpElevator.MI_Monitor_ArchipelagoSpElevator"))))
    (:then_3
      (bind _outactors_4 (Actor|GetAllActorsOfClass "/Game/FactoryGame/Buildable/Factory/TradingPost/Build_TradingPost.Build_TradingPost_C"))
      (for _array_element_4 _outactors_4
        (if (.ReturnValue (Utilities|Map|Find (Variables|Default|GetStage%20to%20MI%20Slot%20Index) (Variables|/Script/Engine.StaticMeshComponent|GetStaticMesh (Variables|/Game/FactoryGame/Buildable/Factory/TradingPost/Build_TradingPost.Build_TradingPost_C|GetMainMesh _array_element_4))))
          (if (== (Rendering|Material|GetMaterial (Variables|/Game/FactoryGame/Buildable/Factory/TradingPost/Build_TradingPost.Build_TradingPost_C|GetMainMesh _array_element_4) (.Value (Utilities|Map|Find (Variables|Default|GetStage%20to%20MI%20Slot%20Index) (Variables|/Script/Engine.StaticMeshComponent|GetStaticMesh (Variables|/Game/FactoryGame/Buildable/Factory/TradingPost/Build_TradingPost.Build_TradingPost_C|GetMainMesh _array_element_4))))) "/Game/FactoryGame/Buildable/Factory/TradingPost/Material/Monitor_HubInside.Monitor_HubInside")
            (Rendering|Material|SetMaterial (Variables|/Game/FactoryGame/Buildable/Factory/TradingPost/Build_TradingPost.Build_TradingPost_C|GetMainMesh _array_element_4) (.Value (Utilities|Map|Find (Variables|Default|GetStage%20to%20MI%20Slot%20Index) (Variables|/Script/Engine.StaticMeshComponent|GetStaticMesh (Variables|/Game/FactoryGame/Buildable/Factory/TradingPost/Build_TradingPost.Build_TradingPost_C|GetMainMesh _array_element_4)))) "/Archipelago/Assets/DerivedArt/Decor/MI_Monitor_ArchipelagoHubInside.MI_Monitor_ArchipelagoHubInside")))))
    (:then_4
      (bind _result (Math|Integer|IncrementInt (Variables|Default|GetTimer%20Ticks))
        (:%20%20
          (if (> _result (Variables|Default|GetMax%20Timer%20Ticks))
            (Utilities|Time|ClearandInvalidateTimerbyHandle (Variables|Default|GetTimer%20Handle))))))))

(event Custom|Start%20Material%20Replacer%20Timer
  (Variables|Default|SetTimer%20Ticks 0)
  (bind _returnvalue (Utilities|Time|SetTimerbyEvent (delegate Custom|Material%20Replacer%20Timer%20Tick) 1.0 true))
  (Variables|Default|SetTimer%20Handle _returnvalue))

(event EventBeginPlay
  (bind _returnvalue (Class|FGBuildableSubsystem|Get))
  (Class|BlueprintLoggingLibrary|LogVerbose "BP_ApDecorSubsystem BeginPlay")
  (Class|FGBlueprintFunctionLibrary|WaitforValidSubsystems)
  (Utilities|IsValid _returnvalue
    (:Is%20Valid
      (EventDispatchers|BindEventtoBuildableConstructedGlobalDelegate _returnvalue (delegate Custom|On%20Buildable%20Constructed))
      (CallFunction|StartMaterialReplacerTimer))))

(fn ConstructionScript)