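; Client-side subsystem that catches Archipelago commands mistakenly typed into Satisfactory chat with the "!" prefix.
; It binds to the chat manager's message-added event and checks whether the latest message is the local player's and starts with "!".
; If so, it posts a yellow hint via SMLRemoteCallObject pointing to the slash prefix and /help.
; Listening is switched off during handling to avoid responding to its own messages.
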(event Custom|On%20Chat%20Message%20Added
  (if (Variables|Default|GetListening)
    ;[1 1 1] Turn off listening when responding (to ensure we NEVER loop responding to ourselves, albeit unlikely)
    (Variables|Default|SetListening false)
    (CallFunction|HandleMessage)
    (Variables|Default|SetListening true)))

(event EventBeginPlay
  (bind _returnvalue (Class|FGChatManager|Get))
  (Utilities|IsValid _returnvalue
    (:Is%20Valid
      (EventDispatchers|BindEventtoOnChatMessageAdded _returnvalue (delegate Custom|On%20Chat%20Message%20Added))
      (Variables|Default|SetListening true)
      (Class|BlueprintLoggingLibrary|LogVerbose "ApAccidentalCommandCatcher Started"))
    (:Is%20Not%20Valid
      (Class|BlueprintLoggingLibrary|LogError "Chat Manager not valid?"))))

(fn ConstructionScript)

(fn GetLatestMessage
  (params (ChatManager :type FG%20Chat%20Manager%20Object%20Reference))
  (bind _messages (LocalVariables|GetMessages))
  (bind _returnvalue (Utilities|Array|LastIndex _messages))
  (bind _output (Utilities|Array|Get(acopy) _messages _returnvalue))
  (bind (_messagetext _messagetype _bislocalplayermessage) (Utilities|Struct|BreakChatMessageStruct _output))
  (Class|FGChatManager|GetReceivedChatMessages ChatManager _messages)
  (return _messagetext _messagetype _bislocalplayermessage))

(fn HandleMessage
  (bind (_message _message_type _is_local_player_message) (CallFunction|GetLatestMessage (Class|FGChatManager|Get)))
  (if _is_local_player_message
    (if (Utilities|String|StartsWith (Utilities|String|ToString(Text) _message) "!")
      (bind _asfgplayer_controller (Utilities|Casting|CastToFGPlayerController (Game|GetPlayerController 0)))
      (Class|SMLRemoteCallObject|SendChatMessage (Class|FGPlayerController|GetRemoteCallObjectOfClass _asfgplayer_controller "/Script/SML.SMLRemoteCallObject") (Utilities|String|ToString(Text) (Utilities|Text|MakeLiteralText "Use the slash ( / ) prefix to run Archipelago commands inside Satisfactory. Use /help for a list of commands.")) (Class|KismetMathLibrary|LinearColorYellow)))))