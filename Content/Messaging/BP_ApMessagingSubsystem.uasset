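; Subsystem that shows Archipelago mod messages in Satisfactory's multiplayer chat.
; On BeginPlay the server queues connection-status messages and, after a delay, warns if Hub 1-1 lacks unlocks, while clients get a local notice.
; Tick drains the join queue, throttled by a Delay, once the chat manager is valid.
; DisplayMessage is server-only and multicasts to a handler that filters each message type through mod config before adding it to chat.
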(event Custom|Multicast%20Display%20Chat%20Message
  (params (Type :type EApMessageType%20Enum :default "ApSystem") (Message :type String) (Color :type Linear%20Color%20Structure%20%28by%20ref%29))
  (bind _asbp_config_property_section (Utilities|Casting|CastToBP_ConfigPropertySection (Class|RuntimeBlueprintFunctionLibrary|ToConfigProperty(ModConfiguration) "/Archipelago/ApConfiguration.ApConfiguration_C")))
  (switch Utilities|FlowControl|Switch|SwitchonEApMessageType Type
    (:ApSystem
      (Class|ApMessagingSubsystem|LocalAddChatMessage Message Color :!label _label))
    (:ItemSend
      (if (Class|RuntimeBlueprintFunctionLibrary|ToBoolean(ConfigProperty) (Class|RuntimeBlueprintFunctionLibrary|ToConfigProperty(ConfigPropertySection) _asbp_config_property_section "ItemSendMessages"))
        (goto _label)))
    (:ItemReceived
      (if (Class|RuntimeBlueprintFunctionLibrary|ToBoolean(ConfigProperty) (Class|RuntimeBlueprintFunctionLibrary|ToConfigProperty(ConfigPropertySection) _asbp_config_property_section "ItemReceivedMessages"))
        (goto _label)))
    (:Hint
      (if (Class|RuntimeBlueprintFunctionLibrary|ToBoolean(ConfigProperty) (Class|RuntimeBlueprintFunctionLibrary|ToConfigProperty(ConfigPropertySection) _asbp_config_property_section "HintMessages"))
        (goto _label)))
    (:Countdown
      (if (Class|RuntimeBlueprintFunctionLibrary|ToBoolean(ConfigProperty) (Class|RuntimeBlueprintFunctionLibrary|ToConfigProperty(ConfigPropertySection) _asbp_config_property_section "CountdownMessages"))
        (goto _label)))
    (:Other
      (if (Class|RuntimeBlueprintFunctionLibrary|ToBoolean(ConfigProperty) (Class|RuntimeBlueprintFunctionLibrary|ToConfigProperty(ConfigPropertySection) _asbp_config_property_section "OtherMessages"))
        (goto _label)))
    (:GiftsReceived
      (if (Class|RuntimeBlueprintFunctionLibrary|ToBoolean(ConfigProperty) (Class|RuntimeBlueprintFunctionLibrary|ToConfigProperty(ConfigPropertySection) _asbp_config_property_section "GiftMessages"))
        (goto _label)))
    (:VaultReceived
      (if (Class|RuntimeBlueprintFunctionLibrary|ToBoolean(ConfigProperty) (Class|RuntimeBlueprintFunctionLibrary|ToConfigProperty(ConfigPropertySection) _asbp_config_property_section "VaultMessages"))
        (goto _label)))))

(event EventBeginPlay
  (|CallParentFunction)
  (Class|BlueprintLoggingLibrary|LogVerbose "BP_ApMessagingSubsystem BeginPlay")
  (if (Ability|HasAuthority)
    (Class|BlueprintLoggingLibrary|LogVerbose "Running with authority")
    (CallFunction|ServerGenerateonJoinMessages) ; Server creates the messages to be displayed on both (listen)server and clients
    (Utilities|FlowControl|Delay 1e+01) ; Bandaid to wait for data to be set up
    (bind _failed_slot_setup (CallFunction|CheckforSlotDataSetupFailure))
    (if _failed_slot_setup
      (Class|ApMessagingSubsystem|DisplayMessage "ApSystem" (Utilities|String|ToString(Text) (Utilities|Text|MakeLiteralText "An error caused slot data creation/loading to fail! Check the HUB for more details. 
 
If you just created this save file, you MUST close this save and create new one - don't keep playing!")) (Class|KismetMathLibrary|LinearColorRed)))
    (else
      (Class|BlueprintLoggingLibrary|LogVerbose "Running on client")
      ;[1 1 1] TODO can we find a way to put this into the normal OnJoinMessages array? but it will cause client/server array length mismatch
      (Utilities|IsValid (Class|FGChatManager|Get) :!label _label
        (:Is%20Valid
          (if (not (Ability|HasAuthority))
            (Class|SMLRemoteCallObject|SendChatMessage (Class|FGPlayerController|GetRemoteCallObjectOfClass (.AsFGPlayer%20Controller (Utilities|Casting|CastToFGPlayerController (Game|GetPlayerController 0))) "/Script/SML.SMLRemoteCallObject") (Utilities|String|ToString(Text) (Utilities|Text|MakeLiteralText "Connected as a Satisfactory multiplayer client to an Archipelago game")) (Class|KismetMathLibrary|LinearColorYellow))))
        (:Is%20Not%20Valid
          (Utilities|FlowControl|Delay 1.0) ; Wait for valid chat manager\nbefore sending any
          (goto _label))))))

(event EventDisplayMessage
  (params (type :type EApMessageType%20Enum :default "ApSystem") (Message :type String) (Color :type Linear%20Color%20Structure%20%28by%20ref%29))
  (Networking|SwitchHasAuthority
    (:Authority
      (CallFunction|MulticastDisplayChatMessage type Message Color))
    (:Remote
      (Class|BlueprintLoggingLibrary|LogError (Utilities|String|Append "Client tried to use DisplayMessage, message was " Message)))))

(event EventTick
  (params (DeltaSeconds :type Float%20%28single-precision%29))
  (bind _onjoinmessages (Variables|Default|GetOnJoinMessages))
  (bind _nextmessageindextodisplay (Variables|Default|GetnextMessageIndexToDisplay))
  (bind _output (Utilities|Array|Get(acopy) _onjoinmessages _nextmessageindextodisplay))
  (|CallParentFunction DeltaSeconds)
  (Utilities|FlowControl|Delay 3.0) ; Limit the rate at which messages are sent
  (Utilities|IsValid (Class|FGChatManager|Get)
    (:Is%20Valid
      (if (Utilities|Array|IsValidIndex _onjoinmessages _nextmessageindextodisplay)
        (Class|ApMessagingSubsystem|DisplayMessage "ApSystem" (.contents _output) (.prefixcolor _output))
        (Class|BlueprintLoggingLibrary|LogVerbose (Utilities|String|ToString(Text) (Utilities|Text|FormatText "Displaying message index {index}: {message}" _nextmessageindextodisplay (.contents _output))))
        (Math|Integer|IncrementInt (Variables|Default|GetnextMessageIndexToDisplay))))
    (:Is%20Not%20Valid
      (Class|BlueprintLoggingLibrary|LogWarning "Chat Manager invalid"))))

(fn ConstructionScript)

(fn SendChatMessagetoAll
  (params (Message :type String) (Color :type Linear%20Color%20Structure))
  (Networking|SwitchHasAuthority
    (:Authority
      (Class|BlueprintLoggingLibrary|LogDisplay (Utilities|String|Append "SendChatMessageToAll: " Message)) ; Also record it in the server logs
      ;[1 1 1] TODO untested, is this off by 1?
      (for _index (range 0 (Class|GameplayStatics|GetNumPlayerControllers))
        (bind _asfgplayer_controller (Utilities|Casting|CastToFGPlayerController (Game|GetPlayerController _index))
          (:then
            (Class|SMLRemoteCallObject|SendChatMessage (Class|FGPlayerController|GetRemoteCallObjectOfClass _asfgplayer_controller "/Script/SML.SMLRemoteCallObject") Message Color))
          (:CastFailed
            (Class|BlueprintLoggingLibrary|LogWarning (Utilities|String|Append "Player controller index " (Utilities|String|ToString(Integer) _index) " was invalid"))))))
    (:Remote
      (Class|BlueprintLoggingLibrary|LogError "SendChatMessageToAll called on client?"))))

(fn ServerGenerateonJoinMessages
  (|ConnectionStatusMessages))

(fn AddonJoinMessage
  (params (Prefix%20Color :type Linear%20Color%20Structure) (Contents :type Text))
  (bind _returnvalue (Utilities|String|ToString(Text) Contents))
  (Utilities|Array|Add (Variables|Default|GetOnJoinMessages) (Utilities|Struct|MakeApStoredChatMessage Prefix%20Color _returnvalue))
  (Class|BlueprintLoggingLibrary|LogVerbose (Utilities|String|Append "Registered message " _returnvalue)))

(fn CheckforSlotDataSetupFailure
  (bind _returnvalue (Class|BlueprintReflectionLibrary|GetClassDefaultObject "/Archipelago/Schematics/AP_HubSchematics/AP_HUB_1_1.AP_HUB_1_1_C"))
  (Class|BlueprintLoggingLibrary|LogVerbose "Checking Hub 1-1 for setup issues")
  (LocalVariables|SetHub%201%201 _returnvalue)
  (if (not (> (Utilities|Array|Length (Variables|/Script/FactoryGame.FGSchematic|GetmUnlocks _returnvalue)) 0))
    (Class|BlueprintLoggingLibrary|LogError "Hub 1-1 has 0 unlocks, setup appears to have failed")
    (Variables|Default|SetIsUnsafeOfflineMode true)
    (return true)))