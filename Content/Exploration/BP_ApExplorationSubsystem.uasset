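; Exploration subsystem that spawns an ApExplorationMarker for every mapped drop pod in the world.
; On BeginPlay it calls PopulateIdToDropPod, then iterates the resulting ID-to-pod map.
; Each marker spawns raised above its pod, receives the ID and pod location as exploration data plus a link to the pod, and is stored in ExplorationMarkers.
; A TODO flags that this data is built here rather than retrieved.
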(event EventBeginPlay
  (bind _idtodroppod (Variables|Default|GetIdToDropPod))
  (Class|BlueprintLoggingLibrary|LogVerbose "BP_ApExplorationSubsystem Begin Play")
  (Class|ApExplorationSubsystem|PopulateIdtoDropPod)
  (bind _keys (Utilities|Map|Keys _idtodroppod))
  (Class|BlueprintLoggingLibrary|LogVerbose (Utilities|String|Append "# markers to spawn: " (Utilities|String|ToString(Integer) (Utilities|Array|Length _keys))))
  (for _array_element _keys
    (bind _returnvalue (Game|SpawnActorfromClass "/Archipelago/Exploration/ApExplorationMarker.ApExplorationMarker_C" (Math|Transform|MakeTransform (+ (Transformation|GetActorLocation (.Value (Utilities|Map|Find _idtodroppod _array_element))) "0.000000,0.000000,450.000000")) "Undefined" 0 (Utilities|Struct|MakeApExplorationData _array_element (Math|Vector|MakeVectorNetQuantize (.X (Math|Vector|BreakVector (Transformation|GetActorLocation (.Value (Utilities|Map|Find _idtodroppod _array_element))))) (.Y (Math|Vector|BreakVector (Transformation|GetActorLocation (.Value (Utilities|Map|Find _idtodroppod _array_element))))) (.Z (Math|Vector|BreakVector (Transformation|GetActorLocation (.Value (Utilities|Map|Find _idtodroppod _array_element))))))) (.Value (Utilities|Map|Find _idtodroppod _array_element)) 0))
    (Utilities|Array|Add (Variables|Default|GetExplorationMarkers) _returnvalue)))

(fn ConstructionScript)