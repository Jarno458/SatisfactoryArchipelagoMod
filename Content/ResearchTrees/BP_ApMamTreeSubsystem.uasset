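; BP_ApMamTreeSubsystem reports which MAM research nodes are currently visible, as a set of IDs taken from schematic menu priorities.
; GetVisibleMamNodeIds scans each unlocked research tree, marking parentless and researched nodes visible, plus the coordinates researched nodes unhide.
; Visible coordinates map back to schematics, whose positive menu priorities become the returned IDs.
; Both research-complete and purchased states are checked because the function can run before the purchase registers.
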(event EventBeginPlay)

(event EventTick
  (params (DeltaSeconds :type Float%20%28single-precision%29)))

(fn ConstructionScript)

(fn GetVisibleMamNodeIds
  (Utilities|Set|Clear (Variables|Default|GetvisibleSchematicIds))
  (bind _array_element (Utilities|ForEachRefLoop (Variables|/Script/FactoryGame.FGResearchManager|GetmUnlockedResearchTrees (Class|FGResearchManager|Get)))
    (:LoopBody
      (bind _returnvalue (Class|FGResearchTree|GetNodes _array_element))
      (Utilities|Set|Clear (Variables|Default|GetvisibleCoordinates))
      (Utilities|Map|Clear (Variables|Default|GetschematicPerCoordinate))
      (bind _array_element_2 (Utilities|ForEachRefLoop _returnvalue)
        (:LoopBody
          (bind _asbpd_research_tree_node (Utilities|Casting|CastToBPD_ResearchTreeNode _array_element_2))
          (Utilities|Map|Add (Variables|Default|GetschematicPerCoordinate) (.Coordinates (Utilities|Struct|BreakMAMTree_NodeData_Struct (Variables|/Game/FactoryGame/Schematics/Research/BPD_ResearchTreeNode.BPD_ResearchTreeNode_C|GetmNodeDataStruct _asbpd_research_tree_node))) (.Schematic (Utilities|Struct|BreakMAMTree_NodeData_Struct (Variables|/Game/FactoryGame/Schematics/Research/BPD_ResearchTreeNode.BPD_ResearchTreeNode_C|GetmNodeDataStruct _asbpd_research_tree_node))))
          (if (or (or (Class|FGResearchManager|IsResearchComplete (Class|FGResearchManager|Get) (.Schematic (Utilities|Struct|BreakMAMTree_NodeData_Struct (Variables|/Game/FactoryGame/Schematics/Research/BPD_ResearchTreeNode.BPD_ResearchTreeNode_C|GetmNodeDataStruct _asbpd_research_tree_node)))) (Class|FGSchematicManager|IsSchematicPurchased (Class|FGSchematicManager|Get) (.Schematic (Utilities|Struct|BreakMAMTree_NodeData_Struct (Variables|/Game/FactoryGame/Schematics/Research/BPD_ResearchTreeNode.BPD_ResearchTreeNode_C|GetmNodeDataStruct _asbpd_research_tree_node))) 0)) (Utilities|Array|IsEmpty (.Parents (Utilities|Struct|BreakMAMTree_NodeData_Struct (Variables|/Game/FactoryGame/Schematics/Research/BPD_ResearchTreeNode.BPD_ResearchTreeNode_C|GetmNodeDataStruct _asbpd_research_tree_node)))))
            (Utilities|Set|Add (Variables|Default|GetvisibleCoordinates) (.Coordinates (Utilities|Struct|BreakMAMTree_NodeData_Struct (Variables|/Game/FactoryGame/Schematics/Research/BPD_ResearchTreeNode.BPD_ResearchTreeNode_C|GetmNodeDataStruct _asbpd_research_tree_node))))
            (if (or (Class|FGResearchManager|IsResearchComplete (Class|FGResearchManager|Get) (.Schematic (Utilities|Struct|BreakMAMTree_NodeData_Struct (Variables|/Game/FactoryGame/Schematics/Research/BPD_ResearchTreeNode.BPD_ResearchTreeNode_C|GetmNodeDataStruct _asbpd_research_tree_node)))) (Class|FGSchematicManager|IsSchematicPurchased (Class|FGSchematicManager|Get) (.Schematic (Utilities|Struct|BreakMAMTree_NodeData_Struct (Variables|/Game/FactoryGame/Schematics/Research/BPD_ResearchTreeNode.BPD_ResearchTreeNode_C|GetmNodeDataStruct _asbpd_research_tree_node))) 0))
              (bind _array_element_3 (Utilities|ForEachRefLoop (.NodesToUnhide (Utilities|Struct|BreakMAMTree_NodeData_Struct (Variables|/Game/FactoryGame/Schematics/Research/BPD_ResearchTreeNode.BPD_ResearchTreeNode_C|GetmNodeDataStruct _asbpd_research_tree_node))))
                (:LoopBody
                  (Utilities|Set|Add (Variables|Default|GetvisibleCoordinates) _array_element_3))))))
        (:Completed
          (bind _result (Utilities|Set|ToArray (Variables|Default|GetvisibleCoordinates)))
          (for _array_element_4 _result
            (if (.ReturnValue (Utilities|Map|Find (Variables|Default|GetschematicPerCoordinate) _array_element_4))
              (if (> (Class|KismetMathLibrary|ToInt64(Float) (Class|FGSchematic|GetMenuPriority (.Value (Utilities|Map|Find (Variables|Default|GetschematicPerCoordinate) _array_element_4)))) 0)
                (Utilities|Set|Add (Variables|Default|GetvisibleSchematicIds) (Class|KismetMathLibrary|ToInt64(Float) (Class|FGSchematic|GetMenuPriority (.Value (Utilities|Map|Find (Variables|Default|GetschematicPerCoordinate) _array_element_4)))))))))))
    (:Completed
      (return (Variables|Default|GetvisibleSchematicIds)))))