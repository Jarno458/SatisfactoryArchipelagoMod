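; Schematic patcher subsystem that swaps the event subsystem's calendar rewards class for the AP Christmas override when the FICSMAS goal is enabled.
; When data becomes available, it caches the original rewards class if not already stored, then applies either the override or that default based on the goal check.
; Its end-play handler writes the cached default back, undoing the patch.
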(event Custom|OnEndPlay_Event
  (params (Actor :type Actor%20Object%20Reference) (EndPlayReason :type EEndPlayReason%20Enum :default "Destroyed"))
  (bind _defaultrewards (Variables|Default|GetdefaultRewards))
  (if (Utilities|IsValidClass _defaultrewards)
    (Variables|/Script/FactoryGame.FGEventSubsystem|SetmCalendarRewardsClass (Class|FGEventSubsystem|GetEventSubsystem) _defaultrewards)))

(event EventBeginPlay)

(event EventTick
  (params (DeltaSeconds :type Float%20%28single-precision%29)))

(fn ConstructionScript)

(fn OnDataAvailable
  (bind _returnvalue (Class|FGEventSubsystem|GetEventSubsystem))
  (if (Utilities|IsValidClass (Variables|Default|GetdefaultRewards))
    _
    (else
      (Variables|Default|SetdefaultRewards (Variables|/Script/FactoryGame.FGEventSubsystem|GetmCalendarRewardsClass (Class|FGEventSubsystem|GetEventSubsystem)))))
  (if (Class|ApSlotDataSubsystem|IsFicsmasGoalEnabled (Class|ApSlotDataSubsystem|Get))
    (Variables|/Script/FactoryGame.FGEventSubsystem|SetmCalendarRewardsClass _returnvalue "/Archipelago/Exploration/APChristmasCalendarRewardsOverride.APChristmasCalendarRewardsOverride_C")
    (else
      (Variables|/Script/FactoryGame.FGEventSubsystem|SetmCalendarRewardsClass _returnvalue (Variables|Default|GetdefaultRewards))))
  (return))