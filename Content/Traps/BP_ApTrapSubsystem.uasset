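; Subsystem that spawns named traps, or the occasional nice surprise, on a given player or on all players when none is given.
; SpawnTrap looks names up in TrapTypes, routing pickup classes to predefined item drops and spawning other classes at an offset from the pawn.
; Classless names run custom logic: a crab ring parented to an existing hatcher, or tamed doggos carrying attached gifts.
; Targets receive chat notices.
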(event EventBeginPlay
  (Class|BlueprintLoggingLibrary|LogVerbose "ApTrapSubsystem Initialize"))

(event EventTick
  (params (DeltaSeconds :type Float%20%28single-precision%29)))

(fn ConstructionScript)

(fn SpawnItemTrap
  (params (item :type FG%20Item%20Descriptor%20Class%20Reference) (quantity :type Integer) (targetPlayer :type Player%20State%20Object%20Reference))
  (bind _returnvalue (PlayerState|GetPawn targetPlayer))
  (if (Utilities|IsValidClass item)
    (if (> quantity 0)
      (Utilities|IsValid targetPlayer
        (:Is%20Valid
          (Utilities|IsValid _returnvalue
            (:Is%20Valid
              (bind _returnvalue_2 (Class|FGItemPickupSpawnable|AddItemtoWorldStackatLocation 0 (Class|FGInventoryLibrary|MakeInventoryStack quantity (Class|FGInventoryLibrary|MakeInventoryItem item)) (Transformation|GetActorLocation _returnvalue) "0, 0, 0" "/Game/FactoryGame/Resource/BP_ItemPickup_Spawnable.BP_ItemPickup_Spawnable_C"))
              (Utilities|IsValid _returnvalue_2
                (:Is%20Valid
                  (return true))
                (:Is%20Not%20Valid
                  (Class|BlueprintLoggingLibrary|LogError "Failed to spawn item pickup?"))))
            (:Is%20Not%20Valid
              (Class|BlueprintLoggingLibrary|LogError (Utilities|String|Append "PlayerState had no pawn: " (Utilities|GetDisplayName targetPlayer))))))
        (:Is%20Not%20Valid
          (Class|BlueprintLoggingLibrary|LogError "Target Player State is not valid")))
      (else
        (Class|BlueprintLoggingLibrary|LogError "Tried to spawn item trap of <1 item")))
    (else
      (Class|BlueprintLoggingLibrary|LogError "Tried to spawn item trap with invalid item class"))))

(fn SpawnTrap
  (params (trapName :type Name :default "None") (targetPlayer :type Player%20State%20Object%20Reference))
  (bind _returnvalue (Utilities|String|ToString(Name) trapName))
  (bind _traptypes (Variables|Default|GetTrapTypes))
  (bind _predefineditemtraps (Variables|Default|GetPredefinedItemTraps))
  (bind (_value _returnvalue_2) (Utilities|Map|Find _traptypes trapName))
  (bind (_value_2 _returnvalue_3) (Utilities|Map|Find _predefineditemtraps trapName))
  (if _returnvalue_2
    (Class|BlueprintLoggingLibrary|LogVerbose (Utilities|String|Append "Spawning trap " _returnvalue))
    ;[1 1 1] TODO do we want to queue traps to wait until there is a valid target?
    (bind (_success _targets) (CallFunction|GatherTargetPlayers targetPlayer))
    (if _success
      (for _array_element _targets
        (Utilities|FlowControl|Sequence
          (:then_0
            (bind _output_get (LocalVariables|SetTarget%20Pawn _array_element))
            (LocalVariables|SetSpawn%20Transform (Math|Transform|MakeTransform (+ (Transformation|GetActorLocation _output_get) (Variables|Default|GetTrap%20Spawn%20Height%20Offset))))
            (if (Utilities|IsValidClass _value)
              ;[1 1 1] Forward item traps to that function
              (Utilities|Casting|CastToBP_PickupClass _value
                (:then
                  (if _returnvalue_3
                    (bind _returnvalue_4 (CallFunction|SpawnItemTrap (.itemclass _value_2) (.amount _value_2) (Variables|/Script/Engine.Pawn|GetPlayerState _output_get)))
                    (if (not _returnvalue_4)
                      (LocalVariables|SetFailed%20on%20At%20Least%20One true))
                    (else
                      (Class|BlueprintLoggingLibrary|LogError (Utilities|String|Append "Invalid predefined item trap: " (Utilities|String|ToString(Name) trapName)))
                      (LocalVariables|SetFailed%20on%20At%20Least%20One true))))
                (:CastFailed
                  ;[1 1 1] Simple Traps
                  (bind _returnvalue_5 (Game|SpawnActorfromClass _value (LocalVariables|GetSpawn%20Transform) "AdjustIfPossibleButAlwaysSpawn" 0 0))
                  (Utilities|IsValid _returnvalue_5
                    (:Is%20Valid
                      (Class|BlueprintLoggingLibrary|LogVerbose (Utilities|String|Append "Spawn " (Utilities|GetDisplayName _returnvalue_5) " on " (Utilities|GetDisplayName (LocalVariables|GetTarget%20Pawn)))))
                    (:Is%20Not%20Valid
                      (LocalVariables|SetFailed%20on%20At%20Least%20One true)
                      (Class|BlueprintLoggingLibrary|LogWarning (Utilities|String|Append "Failed to " (Utilities|String|Append "Spawn " (Utilities|GetDisplayName _returnvalue_5) " on " (Utilities|GetDisplayName (LocalVariables|GetTarget%20Pawn)))))))))
              (else
                ;[1 1 1] Custom Traps
                (switch name trapName
                  (:Default
                    (Class|BlueprintLoggingLibrary|LogError (Utilities|String|Append "No implementation present for trap type " (Utilities|String|ToString(Name) trapName)))
                    (LocalVariables|SetFailed%20on%20At%20Least%20One true))
                  (:TheBees
                    (bind _success_2 (CallFunction|SpawnCrabTrab (LocalVariables|GetSpawn%20Transform)))
                    (if (not _success_2)
                      (LocalVariables|SetFailed%20on%20At%20Least%20One true)))
                  (:DoggoGiftPulseNobelisk
                    (bind (_success_3 _spawned_doggo _spawned_gifts) (CallFunction|SpawnGiftDoggo (LocalVariables|GetSpawn%20Transform) (LocalVariables|GetTarget%20Pawn) "Bouncy Boi" "tongue_03" "1.000000,1.000000,1.000000" "/Game/FactoryGame/Equipment/NobeliskDetonator/Ammo/BP_NobeliskShockwave.BP_NobeliskShockwave_C" 5))
                    (if _success_3
                      ;;[1 1 1] Skeletal mesh is not part of a parent class + for some reason each one needs different scale and position offsets to look right
                      (for _array_element_2 _spawned_gifts
                        (bind _asbp_nobelisk_shockwave (Utilities|Casting|CastToBP_NobeliskShockwave _array_element_2))
                        (Transformation|SetWorldScale3D (Variables|/Game/FactoryGame/Equipment/NobeliskDetonator/Ammo/BP_NobeliskShockwave.BP_NobeliskShockwave_C|GetNobelisExplosive_Skel _asbp_nobelisk_shockwave) "0.500000,0.500000,0.500000")
                        (Transformation|SetRelativeLocation (Variables|/Game/FactoryGame/Equipment/NobeliskDetonator/Ammo/BP_NobeliskShockwave.BP_NobeliskShockwave_C|GetNobelisExplosive_Skel _asbp_nobelisk_shockwave) "2.500000,0.000000,0.000000" false true)
                        (Transformation|SetRelativeRotation (Variables|/Game/FactoryGame/Equipment/NobeliskDetonator/Ammo/BP_NobeliskShockwave.BP_NobeliskShockwave_C|GetNobelisExplosive_Skel _asbp_nobelisk_shockwave) "0.000000,90.000000,0.000000" false false)
                        (Transformation|SetWorldScale3D (Class|FGProjectile|GetCollisionSphere _asbp_nobelisk_shockwave) "3.000000,3.000000,3.000000"))
                      (else
                        (LocalVariables|SetFailed%20on%20At%20Least%20One true))))
                  (:DoggoGiftNukeNobelisk
                    (bind (_success_4 _spawned_doggo_2 _spawned_gifts_2) (CallFunction|SpawnGiftDoggo (LocalVariables|GetSpawn%20Transform) (LocalVariables|GetTarget%20Pawn) "Positively Glowing" "tongue_03" "1.000000,1.000000,1.000000" "/Game/FactoryGame/Equipment/NobeliskDetonator/Ammo/BP_NobeliskNuke.BP_NobeliskNuke_C" 1))
                    (if _success_4
                      (for _array_element_3 _spawned_gifts_2
                        ;;;[1 1 1] TODO no initial blast explosion damage for some reason?
                        (bind _asbp_nobelisk_nuke (Utilities|Casting|CastToBP_NobeliskNuke _array_element_3))
                        (Transformation|SetWorldScale3D (Variables|/Game/FactoryGame/Equipment/NobeliskDetonator/Ammo/BP_NobeliskNuke.BP_NobeliskNuke_C|GetNobelisExplosive_Skel _asbp_nobelisk_nuke) "1.000000,1.000000,1.000000")
                        (Transformation|SetRelativeLocation (Variables|/Game/FactoryGame/Equipment/NobeliskDetonator/Ammo/BP_NobeliskNuke.BP_NobeliskNuke_C|GetNobelisExplosive_Skel _asbp_nobelisk_nuke) "15.000000,0.000000,0.000000" false true)
                        (Transformation|SetRelativeRotation (Variables|/Game/FactoryGame/Equipment/NobeliskDetonator/Ammo/BP_NobeliskNuke.BP_NobeliskNuke_C|GetNobelisExplosive_Skel _asbp_nobelisk_nuke) "0.000000,90.000000,0.000000" false false)
                        (Transformation|SetWorldScale3D (Class|FGProjectile|GetCollisionSphere _asbp_nobelisk_nuke) "1.500000,1.500000,1.500000"))
                      (else
                        (LocalVariables|SetFailed%20on%20At%20Least%20One true))))
                  (:DoggoGiftGasNobelisk
                    (bind (_success_5 _spawned_doggo_3 _spawned_gifts_3) (CallFunction|SpawnGiftDoggo (LocalVariables|GetSpawn%20Transform) (LocalVariables|GetTarget%20Pawn) "Sir Gaseous III" "tongue_03" "1.000000,1.000000,1.000000" "/Game/FactoryGame/Equipment/NobeliskDetonator/Ammo/BP_NobeliskGas.BP_NobeliskGas_C" 1)) ; Small so doggo can escape the cloud alive
                    (if _success_5
                      (for _array_element_4 _spawned_gifts_3
                        (bind _asbp_nobelisk_gas (Utilities|Casting|CastToBP_NobeliskGas _array_element_4))
                        (Transformation|SetWorldScale3D (Variables|/Game/FactoryGame/Equipment/NobeliskDetonator/Ammo/BP_NobeliskGas.BP_NobeliskGas_C|GetNobelisExplosive_Skel _asbp_nobelisk_gas) "3.000000,3.000000,3.000000")
                        (Transformation|SetRelativeLocation (Variables|/Game/FactoryGame/Equipment/NobeliskDetonator/Ammo/BP_NobeliskGas.BP_NobeliskGas_C|GetNobelisExplosive_Skel _asbp_nobelisk_gas) "60.000000,0.000000,0.000000" false true)
                        (Transformation|SetRelativeRotation (Variables|/Game/FactoryGame/Equipment/NobeliskDetonator/Ammo/BP_NobeliskGas.BP_NobeliskGas_C|GetNobelisExplosive_Skel _asbp_nobelisk_gas) "0.000000,90.000000,0.000000" false false)
                        (Transformation|SetWorldScale3D (Class|FGProjectile|GetCollisionSphere _asbp_nobelisk_gas) "0.500000,0.500000,0.500000"))
                      (else
                        (LocalVariables|SetFailed%20on%20At%20Least%20One true))))
                  (:DoggoGiftSlug_Nice
                    (LocalVariables|SetIs%20Nice%20Trap true)
                    (bind (_success_6 _spawned_doggo_4 _spawned_gifts_4) (CallFunction|SpawnGiftDoggo (LocalVariables|GetSpawn%20Transform) (LocalVariables|GetTarget%20Pawn) "Sluggy Buddy" "neck" "1.000000,1.000000,1.000000" "/Game/FactoryGame/Resource/Environment/Crystal/BP_Crystal.BP_Crystal_C" 1))
                    (if _success_6
                      (for _array_element_5 _spawned_gifts_4
                        ;;[1 1 1] Needs to be attached again after being made mobile
                        (bind _asbp_crystal (Utilities|Casting|CastToBP_Crystal _array_element_5))
                        (Components|StaticMesh|SetStaticMesh (Variables|/Game/FactoryGame/Resource/BP_Pickup.BP_Pickup_C|GetStaticMesh _asbp_crystal) "/Game/FactoryGame/Character/Creature/Wildlife/PowerSnail/Mesh/PowerSnail.PowerSnail")
                        (Transformation|SetMobility (Variables|/Game/FactoryGame/Resource/BP_Pickup.BP_Pickup_C|GetStaticMesh _asbp_crystal) "Movable")
                        (Transformation|AttachActorToActor _asbp_crystal _spawned_doggo_4 "scale_05" "SnapToTarget" "SnapToTarget" "KeepRelative" true)
                        (Collision|SetCollisionProfileName (Variables|/Game/FactoryGame/Resource/BP_Pickup.BP_Pickup_C|GetStaticMesh _asbp_crystal) "InteractableFoliageNoCollision" true :!class /Script/Engine.PrimitiveComponent) ; Make it so the doggo can still walk but\nplayers can still collect the slug
                        (Transformation|SetRelativeLocation (Variables|/Game/FactoryGame/Resource/BP_Pickup.BP_Pickup_C|GetStaticMesh _asbp_crystal) "-50.000000,0.000000,0.000000" false true))
                      (else
                        (LocalVariables|SetFailed%20on%20At%20Least%20One true))))))))
          (:then_1
            (CallFunction|SendChatMessage (Variables|/Script/Engine.Pawn|GetPlayerState _array_element) (select (LocalVariables|GetIs%20Nice%20Trap) "A surprise appeard!" "A trap was triggered!") "(R=0.000000,G=1.000000,B=0.000000,A=1.000000)"))))
      (return (not (LocalVariables|GetFailed%20on%20At%20Least%20One)))
      (else
        (Class|BlueprintLoggingLibrary|LogError "No targets were found to recieve the trap")))
    (else
      (Class|BlueprintLoggingLibrary|LogError (Utilities|String|Append "Invalid trap type: " _returnvalue)))))

(fn GatherTargetPlayers
  (params (In%20Target%20Player :type Player%20State%20Object%20Reference))
  (bind _returnvalue (Game|GetPlayerController In%20Target%20Player))
  (bind _to_return (LocalVariables|GetTo%20Return))
  (bind _returnvalue_2 (Pawn|GetControlledPawn _returnvalue))
  (Utilities|FlowControl|Sequence
    (:then_0
      (Utilities|IsValid In%20Target%20Player
        (:Is%20Valid
          (Utilities|IsValid _returnvalue_2
            (:Is%20Valid
              (Utilities|Array|Add (LocalVariables|GetTo%20Return) _returnvalue_2))
            (:Is%20Not%20Valid
              (Class|BlueprintLoggingLibrary|LogError (Utilities|String|Append "Target player has no pawn: " (Utilities|GetDisplayName In%20Target%20Player))))))
        (:Is%20Not%20Valid
          (Class|BlueprintLoggingLibrary|LogDisplay "Passed nullptr player, spawning trap on all players")
          (for _array_element (Variables|/Script/Engine.GameStateBase|GetPlayerArray (Game|GetGameState))
            (Utilities|IsValid (Pawn|GetControlledPawn (Game|GetPlayerController _array_element))
              (:Is%20Valid
                (Utilities|Array|Add (LocalVariables|GetTo%20Return) (Pawn|GetControlledPawn (Game|GetPlayerController _array_element))))
              (:Is%20Not%20Valid
                (Class|BlueprintLoggingLibrary|LogWarning (Utilities|String|Append "Target player has no pawn: " (Utilities|GetDisplayName _array_element)))))))))
    (:then_1
      (return (> (Utilities|Array|Length _to_return) 0) _to_return))))

(fn SpawnGiftDoggo
  (params (SpawnTransform :type Transform) (mFriendActor :type Actor%20Object%20Reference) (mDisplayName :type Text) (SocketName :type Name :default "tongue_03") (Scale :type Vector :default "2.000000,2.000000,2.000000") (Gift%20Class :type Actor%20Class%20Reference) (Gift%20Copies :type Integer))
  (bind (_location _rotation) (Math|Transform|BreakTransform SpawnTransform))
  (bind _returnvalue (Game|SpawnActorfromClass "/Game/FactoryGame/Character/Creature/Wildlife/SpaceRabbit/Char_SpaceRabbit.Char_SpaceRabbit_C" SpawnTransform "Undefined" 0 0))
  (Utilities|IsValid _returnvalue
    (:Is%20Valid
      (Variables|/Game/FactoryGame/Character/Creature/Wildlife/SpaceRabbit/Char_SpaceRabbit.Char_SpaceRabbit_C|SetmFriendActor _returnvalue mFriendActor)
      (Default|SetTamed _returnvalue true)
      (Variables|/Game/FactoryGame/Character/Creature/Wildlife/SpaceRabbit/Char_SpaceRabbit.Char_SpaceRabbit_C|SetmDisplayName _returnvalue mDisplayName)
      (LocalVariables|SetDoggo _returnvalue)
      (LocalVariables|SetPayload (Utilities|Array|MakeArray))
      (for _index (range 1 Gift%20Copies)
        (bind _returnvalue_2 (Game|SpawnActorfromClass Gift%20Class (Math|Transform|MakeTransform _location _rotation Scale) "AlwaysSpawn" 0 0))
        (Utilities|IsValid _returnvalue_2
          (:Is%20Valid
            (Utilities|Array|Add (LocalVariables|GetPayload) _returnvalue_2)
            (Utilities|IsValid (Actor|GetComponentbyClass _returnvalue "/Script/Engine.SkeletalMeshComponent")
              (:Is%20Valid
                (Transformation|AttachComponentToComponent _returnvalue_2 (Actor|GetComponentbyClass _returnvalue "/Script/Engine.SkeletalMeshComponent") SocketName "SnapToTarget" "SnapToTarget" "KeepRelative" true)
                (Class|BlueprintLoggingLibrary|LogVerbose "Spawned DoggoGift"))
              (:Is%20Not%20Valid
                (Class|BlueprintLoggingLibrary|LogError "Doggo did not have Skeletal Mesh?")
                (return false 0 0))))
          (:Is%20Not%20Valid
            (Class|BlueprintLoggingLibrary|LogError "Failed to spawn DoggoGift Payload")
            (return false 0 0))))
      (return true (LocalVariables|GetDoggo) (LocalVariables|GetPayload)))
    (:Is%20Not%20Valid
      (Class|BlueprintLoggingLibrary|LogError "Failed to spawn DoggoGift Doggo"))))

(fn SpawnCrabTrab
  (params (Spawn%20Transform :type Transform))
  (bind _returnvalue (Class|KismetSystemLibrary|MakeLiteralInteger 9))
  (bind (_location _rotation _scale) (Math|Transform|BreakTransform Spawn%20Transform))
  (bind _returnvalue_2 (Actor|GetActorOfClass "/Game/FactoryGame/Character/Creature/Enemy/CrabHatcher/Char_CrabHatcher.Char_CrabHatcher_C"))
  (Utilities|IsValid _returnvalue_2
    (:Is%20Valid
      (LocalVariables|SetParentHatcher _returnvalue_2)
      (for _index (range 0 _returnvalue)
        (bind _returnvalue_3 (Game|SpawnActorfromClass "/Game/FactoryGame/Character/Creature/Enemy/Crab/BabyCrab/BP_FlyingBabyCrab.BP_FlyingBabyCrab_C" (Math|Transform|MakeTransform (+ (Math|Vector|RotateVectorAroundAxis "2000.000000,0.000000,0.000000" (* _index (/ (Math|Float|MakeLiteralFloat 3.6e+02) _returnvalue)) "0.000000,0.000000,1.000000") _location) _rotation _scale) "AdjustIfPossibleButAlwaysSpawn" (LocalVariables|GetParentHatcher) 0))
        (Variables|/Game/FactoryGame/Character/Creature/Enemy/Crab/BabyCrab/BP_FlyingBabyCrab.BP_FlyingBabyCrab_C|SetmParentCrabHatcher _returnvalue_3 (LocalVariables|GetParentHatcher)) ; All of the targeting related properties seem to do nothing, \nthis is what actually makes them attack the player
      )
      (return true))
    (:Is%20Not%20Valid
      (Class|BlueprintLoggingLibrary|LogError "Could not find hatcher to make parent of crabs"))))

(fn SendChatMessage
  (params (Player :type Player%20State%20Object%20Reference) (Message :type Text) (Color :type Linear%20Color%20Structure))
  (bind _returnvalue (Utilities|String|ToString(Text) Message))
  (bind _asfgplayer_controller (Utilities|Casting|CastToFGPlayerController (Game|GetPlayerController Player))
    (:then
      (Class|SMLRemoteCallObject|SendChatMessage (Class|FGPlayerController|GetRemoteCallObjectOfClass _asfgplayer_controller "/Script/SML.SMLRemoteCallObject") _returnvalue Color)
      (Class|BlueprintLoggingLibrary|LogDisplay _returnvalue))
    (:CastFailed
      (Class|BlueprintLoggingLibrary|LogWarning (Utilities|String|Append "Couldn't find player controller to send chat message to: '" (Utilities|GetDisplayName Player) "'")))))