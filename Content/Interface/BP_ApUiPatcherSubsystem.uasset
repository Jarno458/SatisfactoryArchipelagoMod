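; Subsystem that patches base game UI to show Archipelago multiworld info in power storage, MAM hard drive, HUB and HUD widgets.
; On BeginPlay it hooks Blueprint widget functions, mostly Construct, then injects or alters child widgets through each target's parent panel or container.
; It also edits the Power Storage class defaults to describe EnergyLink state.
; EnergyLink and messaging subsystems gate the energy display and offline-mode warning.
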(event Custom|On%20BPW%20Game%20Phase%20Info%20Construct
  (params (Object :type Object%20Object%20Reference))
  ;[1 1 1] Add AP info (connection, goal) to player's HUD
  (bind _asbpw_game_phase_info (Utilities|Casting|CastToBPW_GamePhaseInfo Object))
  (CallFunction|PatchGamePhaseInfowithAPInfo _asbpw_game_phase_info))

(event Custom|On%20BPW%20Harddrive%20Recipe%20Selector%20Construct
  (params (Object :type Object%20Object%20Reference))
  ;[1 1 1] MAM hard drive selection
  (CallFunction|UpdateBPWHarddriveRecipeSelector Object))

(event Custom|On%20BPW%20Harddrive%20Recipe%20Selector%20UpdateUnlockButtons
  (params (Object :type Object%20Object%20Reference))
  ;[1 1 1] MAM hard drive selection
  (CallFunction|UpdateBPWHarddriveRecipeSelector Object))

(event Custom|On%20BPW%20Hub%20Construct
  (params (Object :type Object%20Object%20Reference))
  ;[1 1 1] HUB connection status warning
  (bind _asbpw_hub (Utilities|Casting|CastToBPW_Hub Object))
  (CallFunction|PatchBPWHUBwithSetupWarning _asbpw_hub))

(event Custom|On%20BPW%20Power%20Storage%20Construct
  (params (Object :type Object%20Object%20Reference))
  ;[1 1 1] Power Storage Energy Link
  (bind _asbpw_power_storage (Utilities|Casting|CastToBPW_PowerStorage Object))
  (CallFunction|PatchBPWPowerStorage _asbpw_power_storage))

(event Custom|On%20BPW%20MAM%20Hard%20Drive%20Scanner%20Construct
  (params (Object :type Object%20Object%20Reference))
  ;[1 1 1] MAM Hard Drive scanner main screen
  (bind _asbpw_mam_hard_drive_scanner (Utilities|Casting|CastToBPW_MAM_HardDriveScanner Object))
  (CallFunction|PatchBPWMAMHardDriveScanner _asbpw_mam_hard_drive_scanner))

(event EventBeginPlay
  (Class|BlueprintLoggingLibrary|LogVerbose "ApUiPatcherSubsystem begin")
  ;[1 1 1] Power Storage Energy Link
  (CallFunction|UpdatePowerStorageDescriptorDetails)
  (Class|RuntimeBlueprintFunctionLibrary|BindonBPFunction "/Game/FactoryGame/Buildable/Factory/PowerStorage/UI/BPW_PowerStorage.BPW_PowerStorage_C" (delegate Custom|On%20BPW%20Power%20Storage%20Construct) "Construct" false)
  ;[1 1 1] MAM hard drive selection
  (Class|RuntimeBlueprintFunctionLibrary|BindonBPFunction "/Game/FactoryGame/Buildable/-Shared/WorkBench/BPW_HarddriveRecipeSelector.BPW_HarddriveRecipeSelector_C" (delegate Custom|On%20BPW%20Harddrive%20Recipe%20Selector%20Construct) "Construct" false)
  (Class|RuntimeBlueprintFunctionLibrary|BindonBPFunction "/Game/FactoryGame/Buildable/-Shared/WorkBench/BPW_HarddriveRecipeSelector.BPW_HarddriveRecipeSelector_C" (delegate Custom|On%20BPW%20Harddrive%20Recipe%20Selector%20UpdateUnlockButtons) "UpdateUnlockButtons" false)
  ;[1 1 1] MAM Hard Drive scanner main screen
  (Class|RuntimeBlueprintFunctionLibrary|BindonBPFunction "/Game/FactoryGame/Buildable/-Shared/WorkBench/BPW_MAM_HardDriveScanner.BPW_MAM_HardDriveScanner_C" (delegate Custom|On%20BPW%20MAM%20Hard%20Drive%20Scanner%20Construct) "Construct" false)
  ;[1 1 1] HUB connection status warning
  (Class|RuntimeBlueprintFunctionLibrary|BindonBPFunction "/Game/FactoryGame/Buildable/Factory/TradingPost/UI/BPW_Hub.BPW_Hub_C" (delegate Custom|On%20BPW%20Hub%20Construct) "Construct" false)
  ;[1 1 1] Add AP info (connection, goal) to player's HUD
  (Class|RuntimeBlueprintFunctionLibrary|BindonBPFunction "/Game/FactoryGame/Interface/UI/InGame/ShoppingList/BPW_GamePhaseInfo.BPW_GamePhaseInfo_C" (delegate Custom|On%20BPW%20Game%20Phase%20Info%20Construct) "Construct" false))

(fn ConstructionScript)

(fn PatchBPWPowerStorage
  (params (Widget%20to%20Patch :type BPW%20Power%20Storage%20Object%20Reference))
  (bind _returnvalue (Subsystems|GetSubsystemActorManager))
  (bind _bpw_powerstorageinfo (Variables|/Game/FactoryGame/Buildable/Factory/PowerStorage/UI/BPW_PowerStorage.BPW_PowerStorage_C|GetBPW_PowerStorageInfo Widget%20to%20Patch))
  (bind _returnvalue_2 (Class|SubsystemActorManager|GetSubsystemActor _returnvalue "/Script/Archipelago.ApEnergyLinkSubsystem"))
  (bind _returnvalue_3 (Class|ApEnergyLinkSubsystem|IsEnergyLinkEnabled _returnvalue_2))
  (Class|BlueprintLoggingLibrary|LogVerbose (Utilities|String|Append "Modifying power storage widget " (Utilities|GetDisplayName Widget%20to%20Patch)))
  (Utilities|FlowControl|Sequence
    (:then_0
      (bind _ascanvas_panel (Utilities|Casting|CastToCanvasPanel (Widget|GetParent (Variables|/Game/FactoryGame/Buildable/Factory/PowerStorage/UI/BPW_PowerStorage.BPW_PowerStorage_C|GetmPowerCircuitGraph Widget%20to%20Patch)))
        (:then
          (bind _returnvalue_4 (UserInterface|CreateWidget "/Archipelago/Buildings/PowerStorage/Widget_PowerStorage_ApOverlay.Widget_PowerStorage_ApOverlay_C" 0 _returnvalue_3))
          (Class|CanvasPanel|AddChildtoCanvas _ascanvas_panel _returnvalue_4))
        (:CastFailed
          (Class|BlueprintLoggingLibrary|LogError "mPowerCircuitGraph Parent not CanvasPanel?"))))
    (:then_1
      (if _returnvalue_3
        (Widget|SetVisibility _bpw_powerstorageinfo "Hidden")
        (bind _ascanvas_panel_2 (Utilities|Casting|CastToCanvasPanel (Widget|GetParent _bpw_powerstorageinfo))
          (:then
            (bind _returnvalue_5 (UserInterface|CreateWidget "/Archipelago/Buildings/PowerStorage/Widget_PowerStorage_ApEnergyLinkDisplay.Widget_PowerStorage_ApEnergyLinkDisplay_C" 0 (Variables|/Game/FactoryGame/Buildable/Factory/PowerStorage/UI/BPW_PowerStorage.BPW_PowerStorage_C|GetmBuildablePowerStorage Widget%20to%20Patch)))
            (bind _returnvalue_6 (Class|CanvasPanel|AddChildtoCanvas _ascanvas_panel_2 _returnvalue_5))
            (Variables|/Script/UMG.CanvasPanelSlot|SetLayoutData _returnvalue_6 (Variables|/Script/UMG.CanvasPanelSlot|GetLayoutData (Class|WidgetLayoutLibrary|SlotasCanvasSlot _bpw_powerstorageinfo))))
          (:CastFailed
            (Class|BlueprintLoggingLibrary|LogError "PowerStorageInfo Parent not CanvasPanel?")))))))

(fn PatchBPWHarddriveRecipeSelectorButton
  (params (Widget%20to%20Patch :type BPW%20Harddrive%20Recipe%20Selector%20Button%20Object%20Reference))
  (bind _mschematic (Variables|/Game/FactoryGame/Buildable/-Shared/WorkBench/BPW_HarddriveRecipeSelector_Button.BPW_HarddriveRecipeSelector_Button_C|GetmSchematic Widget%20to%20Patch))
  (bind _returnvalue (Class|FGSchematic|GetUnlocks _mschematic))
  (bind _mrecipecontainer (Variables|/Game/FactoryGame/Buildable/-Shared/WorkBench/BPW_HarddriveRecipeSelector_Button.BPW_HarddriveRecipeSelector_Button_C|GetmRecipeContainer Widget%20to%20Patch))
  (bind _output (Utilities|Array|Get(acopy) _returnvalue))
  (Class|BlueprintLoggingLibrary|LogVerbose (Utilities|String|ToString(Text) (Utilities|Text|FormatText "Patching Hard Drive Selector for schematic: '{schematic}' 1st Unlock: '{unlock}'" (Utilities|GetClassDisplayName _mschematic) _output)))
  (bind _asfgunlock_info_only (Utilities|Casting|CastToFGUnlockInfoOnly _output)
    (:then
      (Variables|/Script/UMG.TextBlock|SetText (Variables|/Game/FactoryGame/Buildable/-Shared/WorkBench/BPW_HarddriveRecipeSelector_Button.BPW_HarddriveRecipeSelector_Button_C|GetmUnlockTypeLabel Widget%20to%20Patch) "Archipelago Item")
      (bind _returnvalue_2 (UserInterface|CreateWidget "/Archipelago/Interface/MAM/Widget_HardDriveDescriptionText.Widget_HardDriveDescriptionText_C" 0 (Variables|/Script/FactoryGame.FGUnlockInfoOnly|GetmUnlockDescription _asfgunlock_info_only)))
      (Widget|Panel|ClearChildren _mrecipecontainer)
      (Widget|Panel|AddChild _mrecipecontainer _returnvalue_2))
    (:CastFailed
      (Class|BlueprintLoggingLibrary|LogVerbose "Unlock type not Info Only") ; In case hard drive results from other mods show up
    )))

(fn UpdateBPWHarddriveRecipeSelector
  (params (Widget%20to%20Patch :type Object%20Object%20Reference))
  (bind _asbpw_harddrive_recipe_selector (Utilities|Casting|CastToBPW_HarddriveRecipeSelector Widget%20to%20Patch))
  (CallFunction|PatchBPWHarddriveRecipeSelectorButton (Variables|/Game/FactoryGame/Buildable/-Shared/WorkBench/BPW_HarddriveRecipeSelector.BPW_HarddriveRecipeSelector_C|GetmUnlockA _asbpw_harddrive_recipe_selector))
  (CallFunction|PatchBPWHarddriveRecipeSelectorButton (Variables|/Game/FactoryGame/Buildable/-Shared/WorkBench/BPW_HarddriveRecipeSelector.BPW_HarddriveRecipeSelector_C|GetmUnlockB _asbpw_harddrive_recipe_selector)))

(fn PatchBPWMAMHardDriveScanner
  (params (Widget%20to%20Patch :type BPW%20MAM%20Hard%20Drive%20Scanner%20Object%20Reference))
  (Class|BlueprintLoggingLibrary|LogVerbose (Utilities|String|Append "Patching hard drive scanner " (Utilities|GetDisplayName Widget%20to%20Patch)))
  (bind _ascanvas_panel (Utilities|Casting|CastToCanvasPanel (Widget|GetParent (Variables|/Game/FactoryGame/Buildable/-Shared/WorkBench/BPW_MAM_HardDriveScanner.BPW_MAM_HardDriveScanner_C|GetmScanButton Widget%20to%20Patch)))
    (:then
      (bind _returnvalue (UserInterface|CreateWidget "/Archipelago/Interface/MAM/Widget_ApHardDriveInfo.Widget_ApHardDriveInfo_C"))
      (bind _returnvalue_2 (Class|CanvasPanel|AddChildtoCanvas _ascanvas_panel _returnvalue))
      (Class|CanvasPanelSlot|SetSize _returnvalue_2 "(X=188.000000,Y=66.000000)")
      (Class|CanvasPanelSlot|SetPosition _returnvalue_2 "(X=605.000000,Y=175.000000)"))
    (:CastFailed
      (Class|BlueprintLoggingLibrary|LogError "Scan Button parent wasn't CanvasPanel?"))))

(fn UpdatePowerStorageDescriptorDetails
  (bind _returnvalue (Class|BlueprintReflectionLibrary|GetClassDefaultObject "/Game/FactoryGame/Buildable/Factory/PowerStorage/Build_PowerStorageMk1.Build_PowerStorageMk1_C"))
  (Variables|/Script/FactoryGame.FGBuildable|SetmDisplayName _returnvalue (Utilities|Text|FormatText "{VanillaPowerStorageName} - EnergyLink" (Variables|/Script/FactoryGame.FGBuildable|GetmDisplayName _returnvalue)))
  (Variables|/Script/FactoryGame.FGBuildable|SetmDescription _returnvalue (Utilities|Text|FormatText "{VanillaPowerStorageDescription} 
 
{ArchipelagoEnergyLinkInformation}" (Variables|/Script/FactoryGame.FGBuildable|GetmDescription _returnvalue) (select (Class|ApEnergyLinkSubsystem|IsEnergyLinkEnabled (Class|SubsystemActorManager|GetSubsystemActor (Subsystems|GetSubsystemActorManager) "/Script/Archipelago.ApEnergyLinkSubsystem")) "Your Archipelago slot has Energy Link enabled! All Power Storage buildings have been augmented with the ability to draw from and contribute to a multiworld energy storage." "Your Archipelago slot does not have Energy Link enabled, so this Power Storage is using its normal base game behavior.")))
  (Class|BlueprintLoggingLibrary|LogVerbose "Updated Power Storage building descriptor with EnergyLink info"))

(fn PatchBPWHUBwithSetupWarning
  (params (Widget%20to%20Patch :type BPW%20Hub%20Object%20Reference))
  (bind _mrewardscontainer (Variables|/Game/FactoryGame/Buildable/Factory/TradingPost/UI/BPW_Hub.BPW_Hub_C|GetmRewardsContainer Widget%20to%20Patch))
  (bind _returnvalue (Class|WidgetLayoutLibrary|SlotasCanvasSlot _mrewardscontainer))
  (if (Variables|/Archipelago/Messaging/BP_ApMessagingSubsystem.BP_ApMessagingSubsystem_C|GetIsUnsafeOfflineMode (Class|SubsystemActorManager|GetSubsystemActor (Subsystems|GetSubsystemActorManager) "/Archipelago/Messaging/BP_ApMessagingSubsystem.BP_ApMessagingSubsystem_C"))
    (Class|BlueprintLoggingLibrary|LogWarning "Displaying unsafe offline mode warning")
    (bind _ascanvas_panel (Utilities|Casting|CastToCanvasPanel (Widget|GetParent _mrewardscontainer))
      (:then
        (bind _returnvalue_2 (UserInterface|CreateWidget "/Archipelago/Interface/HUB/Widget_Inject_HUBConnectionWarning.Widget_Inject_HUBConnectionWarning_C" (Widget|GetOwningPlayer _ascanvas_panel)))
        (bind _returnvalue_3 (Class|CanvasPanel|AddChildtoCanvas _ascanvas_panel _returnvalue_2))
        (Class|CanvasPanelSlot|SetAnchors _returnvalue_3 (Class|CanvasPanelSlot|GetAnchors _returnvalue))
        (Class|CanvasPanelSlot|SetOffsets _returnvalue_3 (Class|CanvasPanelSlot|GetOffsets _returnvalue))
        (Class|CanvasPanelSlot|SetPosition _returnvalue_3 (Class|CanvasPanelSlot|GetPosition _returnvalue)))
      (:CastFailed
        (Class|BlueprintLoggingLibrary|LogError "TPost MRewardsContainer parent not Overlay?")))))

(fn PatchGamePhaseInfowithAPInfo
  (params (Widget%20to%20Patch :type BPW%20Game%20Phase%20Info%20Object%20Reference))
  (bind _asvertical_box (Utilities|Casting|CastToVerticalBox (Widget|GetParent (Variables|/Game/FactoryGame/Interface/UI/InGame/ShoppingList/BPW_GamePhaseInfo.BPW_GamePhaseInfo_C|GetmCurrentPhaseCostBox Widget%20to%20Patch)))
    (:then
      (LocalVariables|SetmCurrentPhaseCostBox _asvertical_box)
      (Utilities|FlowControl|Sequence
        (:then_0
          (bind _returnvalue (UserInterface|CreateWidget "/Archipelago/Interface/HUD/Widget_Inject_HUDConnectionInfo.Widget_Inject_HUDConnectionInfo_C"))
          (Class|VerticalBox|AddChildtoVerticalBox (LocalVariables|GetmCurrentPhaseCostBox) _returnvalue))))
    (:CastFailed
      (Class|BlueprintLoggingLibrary|LogError "mCurrentPhaseCostBox Was not VerticalBox"))))